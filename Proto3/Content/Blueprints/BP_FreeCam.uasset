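; BP_FreeCam is a free camera with pan, orbit and zoom, driven by Enhanced Input and mouse wheel keys.
; Move input offsets the Pivot locally; while orbit is held, the cursor hides and look input yaws the Pivot and pitches the SpringArm.
; The pitch clamp limits each input delta, not the accumulated angle.
; The wheel scales arm length multiplicatively within near and far limits.
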(event `self.ReceiveBeginPlay`
  (bind _returnvalue (`GameplayStatics.GetPlayerController` 0))
  ; Enables input.
  (`EnhancedInputSubsystemInterface.AddMappingContext` (pcsubsystem `EnhancedInputLocalPlayerSubsystem` _returnvalue) "/Game/Input/IMC_FreeCam.IMC_FreeCam" 0 (struct))
  (`WidgetBlueprintLibrary.SetInputMode_GameAndUIEx` _returnvalue null)
  (set `PlayerController.bShowMouseCursor` true _returnvalue))

(event `EnhancedInput|/Game/Input/IA_Move`
  (params (ActionValue :type "Vector2D Structure") (ElapsedSeconds :type "Float (double-precision)") (TriggeredSeconds :type "Float (double-precision)") (InputAction :type "InputAction Object Reference" :default "/Game/Input/IA_Move.IA_Move"))
  (bind (_x _y) (`KismetMathLibrary.BreakVector2D` ActionValue))
  (bind _cammovespeed (`self.CamMoveSpeed`))
  ; X is Y. Y is X.
  (:`Triggered`
    (`SceneComponent.K2_AddLocalOffset` (`self.Pivot`) (`KismetMathLibrary.MakeVector` (* _y _cammovespeed) (* _x _cammovespeed)) false false)))

(event `EnhancedInput|/Game/Input/IA_Orbit`
  (params (ActionValue :type Boolean) (ElapsedSeconds :type "Float (double-precision)") (TriggeredSeconds :type "Float (double-precision)") (InputAction :type "InputAction Object Reference" :default "/Game/Input/IA_Orbit.IA_Orbit"))
  (bind _returnvalue (`GameplayStatics.GetPlayerController` 0))
  (:`Started`
    (set `self.isOrbit` true)
    (set `PlayerController.bShowMouseCursor` false _returnvalue)
    (`WidgetBlueprintLibrary.SetInputMode_GameOnly` _returnvalue))
  (:`Completed`
    (set `self.isOrbit` false)
    (set `PlayerController.bShowMouseCursor` true _returnvalue)
    (`WidgetBlueprintLibrary.SetInputMode_GameAndUIEx` _returnvalue null)))

(event `EnhancedInput|/Game/Input/IA_Look`
  (params (ActionValue :type "Vector2D Structure") (ElapsedSeconds :type "Float (double-precision)") (TriggeredSeconds :type "Float (double-precision)") (InputAction :type "InputAction Object Reference" :default "/Game/Input/IA_Look.IA_Look"))
  (:`Triggered`
    (if (`self.isOrbit`)
      (`SceneComponent.K2_AddLocalRotation` (`self.Pivot`) (`KismetMathLibrary.MakeRotator` 0.0 0.0 (* ActionValue_X (`self.CamRotMult`))) false false)
      (`SceneComponent.K2_AddLocalRotation` (`self.SpringArm`) (`KismetMathLibrary.MakeRotator` 0.0 (`KismetMathLibrary.FClamp` (* (`self.GetInputAxisKeyValue`) (`self.CamRotMult`)) -80.0 80.0)) false false))))

(event `Key|MouseScrollUp`
  (params (Key :type "Key Structure"))
  (bind _returnvalue (* (`SpringArmComponent.TargetArmLength` (`self.SpringArm`)) 0.5))
  ;[0.6198 0.1504 0.5276 0.5] Zoom in
  (:`Pressed`
    (if (>= _returnvalue (`self.MinArmLength`))
      (set `SpringArmComponent.TargetArmLength` _returnvalue (`self.SpringArm`)))))

(event `Key|MouseScrollDown`
  (params (Key :type "Key Structure"))
  ;[0.6198 0.1504 0.5276 0.5] Zoom out
  (:`Pressed`
    (set `SpringArmComponent.TargetArmLength` (`KismetMathLibrary.FClamp` (* (`SpringArmComponent.TargetArmLength` (`self.SpringArm`)) 1.5) 0.0 1000.0) (`self.SpringArm`))))

(fn `UserConstructionScript`)