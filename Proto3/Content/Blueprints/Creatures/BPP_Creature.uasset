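; Creature actor that builds its look from held traits and can gain traits from nearby environmental features.
; InfluenceRadius overlaps track active features, and a one-second looping timer rolls each one's chance to pass its trait.
; InitiateAppearance applies base materials, then trait-driven meshes, eye decals and materials; InitiateCreature also sets name and label.
; Hover shows an overlay outline, and clicking makes it the spectated view target with an orbit camera.
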(event `self.ReceiveActorBeginCursorOver`
  ; Highlight Outline
  (for _array_element (`self.K2_GetComponentsByClass` "/Script/Engine.MeshComponent")
    (`MeshComponent.SetOverlayMaterial` _array_element "/Game/Assets/Materials/M_HighlightOutline.M_HighlightOutline")))

(event `self.ReceiveActorOnClicked`
  (params (ButtonPressed :type "Key Structure"))
  (bind _asbp_player_controller (cast `/Game/Blueprints/BP_PlayerController` (`GameplayStatics.GetPlayerController` 0)))
  (set `/Game/Blueprints/BP_PlayerController.SpectateCreature` self _asbp_player_controller)
  (`PlayerController.SetViewTargetWithBlend` (`GameplayStatics.GetPlayerController` 0) self 0.0 "VTBlend_Linear" 0.0 false))

(event `self.ReceiveBeginPlay`
  ; Initiate regular check timer
  (`KismetSystemLibrary.K2_SetTimerDelegate` (delegate `RunRegularProcesses`) 1.0 true)
  (set `PlayerController.bEnableClickEvents` true (`GameplayStatics.GetPlayerController` 0)))

(event `self.ReceiveActorEndCursorOver`
  ; Highlight Outline
  (for _array_element (`self.K2_GetComponentsByClass` "/Script/Engine.MeshComponent")
    (`MeshComponent.SetOverlayMaterial` _array_element null)))

(event `RunRegularProcesses`
  ; Check Each Second
  ; Will Environmental Features in radius pass their trait?
  (for _array_element (`self.Active Environmental Influences`)
    (if (<= (`KismetMathLibrary.RandomFloatInRange` 0.0 100.0) (`/Game/Blueprints/Placeables/Environmental_Features/BPP_EnvironmentalFeatures.InfluenceChance` _array_element))
      (`/Game/Blueprints/Placeables/Environmental_Features/BPP_EnvironmentalFeatures.Pass Trait` _array_element self))))

(event `self.Influence Radius.OnComponentBeginOverlap`
  (params (OverlappedComponent :type "PrimitiveComponent Object Reference") (OtherActor :type "Actor Object Reference") (OtherComp :type "PrimitiveComponent Object Reference") (OtherBodyIndex :type Integer) (bFromSweep :type Boolean) (SweepResult :type "HitResult Structure (by ref)"))
  ; Adds environmental features to an array of features within the creature's radius, meaning that they are able to influence the creature
  (if (`self.ActorHasTag` OtherActor "EnvFeature")
    (bind _asbpp_environmental_features (cast `/Game/Blueprints/Placeables/Environmental_Features/BPP_EnvironmentalFeatures` OtherActor))
    (`KismetArrayLibrary.Array_Insert` (`self.Active Environmental Influences`) _asbpp_environmental_features)))

(event `self.Influence Radius.OnComponentEndOverlap`
  (params (OverlappedComponent :type "PrimitiveComponent Object Reference") (OtherActor :type "Actor Object Reference") (OtherComp :type "PrimitiveComponent Object Reference") (OtherBodyIndex :type Integer))
  ; Adds environmental features to an array of features within the creature's radius, meaning that they are able to influence the creature
  (if (`self.ActorHasTag` OtherActor "EnvFeature")
    (bind _asbpp_environmental_features (cast `/Game/Blueprints/Placeables/Environmental_Features/BPP_EnvironmentalFeatures` OtherActor))
    (`KismetArrayLibrary.Array_RemoveItem` (`self.Active Environmental Influences`) _asbpp_environmental_features)))

(fn `CreatureHighlight`
  (params (True :type Boolean))
  (for _array_element (`self.K2_GetComponentsByClass` "/Script/Engine.StaticMeshComponent")
    (`PrimitiveComponent.SetCustomDepthStencilValue` _array_element 1)
    (`PrimitiveComponent.SetRenderCustomDepth` _array_element True)))

(fn `Initiate Creature`
  (returns (Name :type String))
  (bind _asgm_main_game_mode (cast `/Game/Blueprints/GM_MainGameMode` (`GameplayStatics.GetGameMode`)))
  (bind _output_get (set `self.CreatureID` (`/Game/Blueprints/GM_MainGameMode.LatestCreatureID` _asgm_main_game_mode)))
  (bind _output_get_2 (set `self.CreatureName` (`KismetTextLibrary.Conv_TextToString` (`|FormatText` "Creature {S}-{ID}" (`self.SpeciesID`) _output_get))))
  (`self.Load Label`)
  ; Check for objects already in radius when spawned
  (bind _outactors (`GameplayStatics.GetAllActorsWithTag` "EnvFeature"))
  (for _array_element _outactors
    (if (`PrimitiveComponent.IsOverlappingActor` (`self.Influence Radius`) _array_element)
      (bind _asbpp_environmental_features (cast `/Game/Blueprints/Placeables/Environmental_Features/BPP_EnvironmentalFeatures` _array_element))
      (`KismetArrayLibrary.Array_Insert` (`self.Active Environmental Influences`) _asbpp_environmental_features)
      (`self.InitiateAppearance` :!label _label)
      (return _output_get_2)))
  (goto _label))

(fn `InitiateAppearance`
  (bind _leg_bl (`self.Leg_BL`))
  (bind _head (`self.Head`))
  (bind _reye (`self.REye`))
  (bind _body (`self.Body`))
  (bind _leg_br (`self.Leg_BR`))
  (bind _leg_fr (`self.Leg_FR`))
  (bind _leg_fl (`self.Leg_FL`))
  (bind (_headtype _headquantity _headsize _headtilt _bodytype _bodylength _bodywidth _bodydepth _armtype _armquantity _armlength _legtype _legquantity _leglength _tailtype _tailquantity _taillength _tailwidth _legwidth _eyetype _eyequantity _headprimarymaterial _headsecondarymaterial _bodymaterial _limbmaterial) (break `/Game/Blueprints/Structures/ThingsTraitsCanChange/ST_CreatureAppearance` (`.CreatureAppearance_6_38D687554A8A0B5D091ADC94206ACA34` (break `/Game/Blueprints/Structures/ST_CreatureBaseValues` (`self.Base Values`)))))
  (`PrimitiveComponent.SetMaterial` (`self.Head`) 0 _headprimarymaterial)
  (`PrimitiveComponent.SetMaterial` (`self.Head`) 1 _headsecondarymaterial)
  (`PrimitiveComponent.SetMaterial` (`self.Body`) 0 _bodymaterial)
  (`PrimitiveComponent.SetMaterial` (`self.Leg_FR`) 0 _limbmaterial)
  (`PrimitiveComponent.SetMaterial` (`self.Leg_BR`) 0 _limbmaterial)
  (`PrimitiveComponent.SetMaterial` (`self.Leg_BL`) 0 _limbmaterial)
  (`PrimitiveComponent.SetMaterial` (`self.Leg_FL`) 0 _limbmaterial)
  (for _array_element (`self.Held Traits`)
    (bind ((`AffectedAttribute_2_D847424143BCB094A3BABF9B0317C67F` _affectedattribute) (`Amount_8_A0371131402D7FB18A3E0B97326AABC4` _amount) (`Material_11_443646404CB2E2BF372DE0A2C1875D4C` _material)) (break `/Game/Blueprints/Structures/ST_TraitOperation` (`.TraitOperation_14_8A1D66F34F2C47D1A185FFA6C73B2473` (break `/Game/Blueprints/Structures/ST_HeldTrait` _array_element))))
    (switch `/Game/Blueprints/Enumeration/Creatures/EN_CreatureAttribute` _affectedattribute
      (:`NewEnumerator9`
        (switch `int` (`KismetMathLibrary.Round` _amount)
          (:`0`
            (`StaticMeshComponent.SetStaticMesh` _head "/Game/Assets/CreatureParts/Head/part_head_1_NOEYES.part_head_1_NOEYES"))
          (:`1`
            (`StaticMeshComponent.SetStaticMesh` _head "/Game/Assets/CreatureParts/Head/part_head_2_NOEYES.part_head_2_NOEYES"))
          (:`2`
            (`StaticMeshComponent.SetStaticMesh` _head "/Game/Assets/CreatureParts/Head/part_head_3_NOEYES.part_head_3_NOEYES"))
          (:`3`
            (`StaticMeshComponent.SetStaticMesh` _head "/Game/Assets/CreatureParts/Head/part_head_4_NOEYES.part_head_4_NOEYES"))))
      (:`NewEnumerator13`
        (switch `int` (`KismetMathLibrary.Round` _amount)
          (:`1`
            (`StaticMeshComponent.SetStaticMesh` _body "/Game/Assets/CreatureParts/Body/part_body_1.part_body_1"))
          (:`2`
            (`StaticMeshComponent.SetStaticMesh` _body "/Game/Assets/CreatureParts/Body/part_body_2.part_body_2"))
          (:`3`
            (`StaticMeshComponent.SetStaticMesh` _body "/Game/Assets/CreatureParts/Body/part_body_3.part_body_3"))))
      (:`NewEnumerator20`
        (switch `int` (`KismetMathLibrary.Round` _amount)
          (:`0`
            (`StaticMeshComponent.SetStaticMesh` _leg_bl "/Game/Assets/CreatureParts/Leg/part_leg_1.part_leg_1")
            (`StaticMeshComponent.SetStaticMesh` _leg_br "/Game/Assets/CreatureParts/Leg/part_leg_1.part_leg_1")
            (`StaticMeshComponent.SetStaticMesh` _leg_fr "/Game/Assets/CreatureParts/Leg/part_leg_1.part_leg_1")
            (`StaticMeshComponent.SetStaticMesh` _leg_fl "/Game/Assets/CreatureParts/Leg/part_leg_1.part_leg_1"))
          (:`1`
            (`StaticMeshComponent.SetStaticMesh` _leg_bl "/Game/Assets/CreatureParts/Leg/part_leg_2.part_leg_2")
            (`StaticMeshComponent.SetStaticMesh` _leg_br "/Game/Assets/CreatureParts/Leg/part_leg_2.part_leg_2")
            (`StaticMeshComponent.SetStaticMesh` _leg_fr "/Game/Assets/CreatureParts/Leg/part_leg_2.part_leg_2")
            (`StaticMeshComponent.SetStaticMesh` _leg_fl "/Game/Assets/CreatureParts/Leg/part_leg_2.part_leg_2"))))
      (:`NewEnumerator28`
        (switch `int` (`KismetMathLibrary.Round` _amount)
          (:`0`
            (`DecalComponent.SetDecalMaterial` _reye "/Game/Assets/CreatureParts/eye/M_eye_Inst1.M_eye_Inst1")
            (`DecalComponent.SetDecalMaterial` (`self.LEye`) "/Game/Assets/CreatureParts/eye/M_eye_Inst1.M_eye_Inst1"))
          (:`1`
            (`DecalComponent.SetDecalMaterial` _reye "/Game/Assets/CreatureParts/eye/M_eye_Inst2.M_eye_Inst2")
            (`DecalComponent.SetDecalMaterial` (`self.LEye`) "/Game/Assets/CreatureParts/eye/M_eye_Inst2.M_eye_Inst2"))
          (:`2`
            (`DecalComponent.SetDecalMaterial` _reye "/Game/Assets/CreatureParts/eye/M_eye_Inst3.M_eye_Inst3")
            (`DecalComponent.SetDecalMaterial` (`self.LEye`) "/Game/Assets/CreatureParts/eye/M_eye_Inst3.M_eye_Inst3"))
          (:`3`
            (`DecalComponent.SetDecalMaterial` _reye "/Game/Assets/CreatureParts/eye/M_eye_Inst4.M_eye_Inst4")
            (`DecalComponent.SetDecalMaterial` (`self.LEye`) "/Game/Assets/CreatureParts/eye/M_eye_Inst4.M_eye_Inst4"))
          (:`4`
            (`DecalComponent.SetDecalMaterial` _reye "/Game/Assets/CreatureParts/eye/M_eye_Inst5.M_eye_Inst5")
            (`DecalComponent.SetDecalMaterial` (`self.LEye`) "/Game/Assets/CreatureParts/eye/M_eye_Inst5.M_eye_Inst5"))
          (:`5`
            (`DecalComponent.SetDecalMaterial` _reye "/Game/Assets/CreatureParts/eye/M_eye_Inst6.M_eye_Inst6")
            (`DecalComponent.SetDecalMaterial` (`self.LEye`) "/Game/Assets/CreatureParts/eye/M_eye_Inst6.M_eye_Inst6"))
          (:`6`
            (`DecalComponent.SetDecalMaterial` _reye "/Game/Assets/CreatureParts/eye/M_eye_Inst7.M_eye_Inst7")
            (`DecalComponent.SetDecalMaterial` (`self.LEye`) "/Game/Assets/CreatureParts/eye/M_eye_Inst7.M_eye_Inst7"))
          (:`7`
            (`DecalComponent.SetDecalMaterial` _reye "/Game/Assets/CreatureParts/eye/M_eye_Inst8.M_eye_Inst8")
            (`DecalComponent.SetDecalMaterial` (`self.LEye`) "/Game/Assets/CreatureParts/eye/M_eye_Inst8.M_eye_Inst8"))))
      (:`NewEnumerator30`
        (`PrimitiveComponent.SetMaterial` (`self.Head`) 0 _material))
      (:`NewEnumerator31`
        (`PrimitiveComponent.SetMaterial` (`self.Head`) 1 _material))
      (:`NewEnumerator32`
        (`PrimitiveComponent.SetMaterial` (`self.Body`) 0 _material))
      (:`NewEnumerator33`
        (`PrimitiveComponent.SetMaterial` (`self.Leg_FR`) 0 _material)
        (`PrimitiveComponent.SetMaterial` (`self.Leg_BR`) 0 _material)
        (`PrimitiveComponent.SetMaterial` (`self.Leg_BL`) 0 _material)
        (`PrimitiveComponent.SetMaterial` (`self.Leg_FL`) 0 _material)))))

(fn `Load Label`
  ; Set Label Values - called when spawned
  (bind _aswbp_creature_labels (cast `/Game/Blueprints/Widgets/WBP_CreatureLabels` (`WidgetComponent.GetWidget` (`self.CreatureLabel`))))
  (set `/Game/Blueprints/Widgets/WBP_CreatureLabels.Generation` (`self.Generation`) _aswbp_creature_labels)
  (set `/Game/Blueprints/Widgets/WBP_CreatureLabels.Species` (`self.SpeciesID`) _aswbp_creature_labels)
  (set `/Game/Blueprints/Widgets/WBP_CreatureLabels.Name` (`self.CreatureName`) _aswbp_creature_labels)
  (set `/Game/Blueprints/Widgets/WBP_CreatureLabels.ID` (`self.CreatureID`) _aswbp_creature_labels))

(fn `OrbitCamera`
  (params (LookX :type "Float (double-precision)") (LookY :type "Float (double-precision)"))
  (`SceneComponent.K2_AddLocalRotation` (`self.CameraPivot`) (`KismetMathLibrary.MakeRotator` 0.0 0.0 LookX) false false)
  (`SceneComponent.K2_AddLocalRotation` (`self.SpringArm`) (`KismetMathLibrary.MakeRotator` 0.0 LookY) false false))

(fn `Recalculate Effective Values`
  (`self.InitiateAppearance`)
  (for _array_element (`self.Held Traits`)
    (switch `/Game/Blueprints/Enumeration/Creatures/EN_CreatureAttribute` (break `/Game/Blueprints/Structures/ST_TraitOperation` (`.TraitOperation_14_8A1D66F34F2C47D1A185FFA6C73B2473` (break `/Game/Blueprints/Structures/ST_HeldTrait` _array_element))))))

(fn `UserConstructionScript`
  (`self.InitiateAppearance`))