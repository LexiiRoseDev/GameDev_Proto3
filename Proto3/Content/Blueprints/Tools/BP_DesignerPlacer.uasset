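; Designer-mode placement tool that previews a selected actor under the mouse cursor and spawns it on left click.
; While GM_MainGameMode has designer mode enabled, Tick moves the root to the cursor's Visibility trace impact point.
; ObjectSelected sets the child actor to the chosen class as a ghost, with actor collision off and preview materials applied.
; Clicking, gated by designer mode, always spawns that class at the preview's transform.
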(event `self.ReceiveTick`
  (params (DeltaSeconds :type "Float (single-precision)"))
  (bind (_hitresult _returnvalue) (`PlayerController.GetHitResultUnderCursorByChannel` (`GameplayStatics.GetPlayerController` 0) "TraceTypeQuery1" true))
  (bind _asgm_main_game_mode (cast `/Game/Blueprints/GM_MainGameMode` (`GameplayStatics.GetGameMode`)))
  (if (`/Game/Blueprints/GM_MainGameMode.DesignerModeEnabled` _asgm_main_game_mode)
    (if _returnvalue
      (`SceneComponent.K2_SetWorldLocation` (`self.DefaultSceneRoot`) (`.ImpactPoint` (`GameplayStatics.BreakHitResult` _hitresult)) false false))))

(event `Key|LeftMouseButton`
  (params (Key :type "Key Structure"))
  (:`Pressed`
    (`self.DesignerModeEnabled?`)
    (`|SpawnActorFromClass` (`self.BlueprintToSpawn`) (`SceneComponent.K2_GetComponentToWorld` (`self.ChildActor`)) "AlwaysSpawn" "MultiplyWithRoot" null null)))

(fn `ObjectSelected`
  (params (`Blueprint Actor` :type "Actor Class Reference"))
  (bind _childactor (`ChildActorComponent.ChildActor` (`self.ChildActor`)))
  (bind _output_get (set `self.BlueprintToSpawn` `Blueprint Actor`))
  (`ChildActorComponent.SetChildActorClass` (`self.ChildActor`) _output_get)
  (`self.SetActorEnableCollision` _childactor false)
  (for _array_element (`self.K2_GetComponentsByClass` _childactor "/Script/Engine.MeshComponent")
    (for _index (range (+ (`PrimitiveComponent.GetNumMaterials` _array_element) 1))
      (`PrimitiveComponent.SetMaterial` _array_element _index "/Game/Assets/Materials/MI_PlacePreviewG.MI_PlacePreviewG"))))

(fn `UserConstructionScript`)