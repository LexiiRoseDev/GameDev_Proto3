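; BP_CreatureSpawner is an actor that scatters a random number of PBP_Creature actors around itself on BeginPlay.
; SpawnCreatures picks a count between configurable bounds, then spawns each at a random XY offset from the root, with fixed world Z, random yaw and slight pitch.
; Spawning adjusts for collisions or fails, and the loop counts only valid spawns, retrying without an attempt limit.
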(event `self.ReceiveBeginPlay`
  (`self.SpawnCreatures`))

(fn `SpawnCreatures`
  (locals (SpawnCount :type Integer) (Spawned :type Integer))
  (bind (_returnvalue_x _returnvalue_y) (`KismetMathLibrary.BreakVector` (`SceneComponent.K2_GetComponentLocation` (`self.DefaultSceneRoot`))))
  (bind _output_get (set `local.SpawnCount` (`KismetMathLibrary.RandomIntegerInRange` (`self.MinSpawnCount`) (`self.MaxSpawnCount`))))
  (while (< (`local.Spawned`) _output_get)
    (bind _returnvalue (`|SpawnActorFromClass` "/Game/Blueprints/Creatures/PBP_Creature.PBP_Creature_C" (`KismetMathLibrary.MakeTransform` (`KismetMathLibrary.MakeVector` (+ _returnvalue_x (`KismetMathLibrary.RandomFloatInRange` -500.0 500.0)) (+ _returnvalue_y (`KismetMathLibrary.RandomFloatInRange` -500.0 500.0)) 1.0) (`KismetMathLibrary.MakeRotator` 0.0 (`KismetMathLibrary.RandomFloatInRange` -1.0 1.0) (`KismetMathLibrary.RandomFloatInRange` 0.0 360.0))) "AdjustIfPossibleButDontSpawnIfColliding" "MultiplyWithRoot" null null))
    (`/Engine/EditorBlueprintResources/StandardMacros.IsValid` _returnvalue
      (:`Is Valid`
        (`/Engine/EditorBlueprintResources/StandardMacros.IncrementInt` (`local.Spawned`))))))

(fn `UserConstructionScript`)