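; AI controller for BPP_Creature that drives random wandering and foraging at berry bushes.
; Wander starts on possession, moves to random reachable points, then uses random delays and a coin flip to either repeat, unless food is being sought, or stop.
; SeekFood picks a random BP_BerryBush, retrying recursively if invalid; arrival raises hunger value, clears the seeking flag and resumes wandering.
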(event `Wander`
  (bind _returnvalue (`self.K2_GetPawn`))
  ; Wander logic, set a point in range to move towards and go there.
  (`|AIMoveTo` _returnvalue (`NavigationSystemV1.K2_GetRandomReachablePointInRadius` (`self.K2_GetActorLocation` _returnvalue) (`self.WanderRadius`) null null) null
    (:`OnSuccess`
      ; Flip a coin, if heads then wander again. If tails, do nothing.
      (`KismetSystemLibrary.Delay` (`KismetMathLibrary.RandomFloatInRange` 1.0 3.0)))
    (:`OnFail`
      _))
  (if (`KismetMathLibrary.RandomBool`)
    (`KismetSystemLibrary.Delay` (`KismetMathLibrary.RandomFloatInRange` 1.0 3.0))
    (if (not (`/Game/Blueprints/Creatures/BPP_Creature.isSeekingFood` (`self.CreatureRef`)))
      (`self.Wander`))))

(event `self.ReceivePossess`
  (params (PossessedPawn :type "Pawn Object Reference"))
  ; Makes them move around on spawn.
  (bind _asbpp_creature (cast `/Game/Blueprints/Creatures/BPP_Creature` PossessedPawn))
  (set `self.CreatureRef` _asbpp_creature)
  (`self.Wander`))

(event `SeekFood`
  (bind _returnvalue (`self.K2_GetPawn`))
  (bind _outactors (`GameplayStatics.GetAllActorsOfClass` "/Game/Blueprints/Placeables/Food_Sources/BP_BerryBush.BP_BerryBush_C"))
  (bind _outitem (`KismetArrayLibrary.Array_Random` _outactors))
  (`/Engine/EditorBlueprintResources/StandardMacros.IsValid` _outitem
    (:`Is Valid`
      (`|AIMoveTo` _returnvalue (0.0 0.0 0.0) _outitem
        (:`OnSuccess`
          (`KismetSystemLibrary.PrintString` "BERRIES!!")
          (bind _asbpp_creature (cast `/Game/Blueprints/Creatures/BPP_Creature` _returnvalue))
          (set `/Game/Blueprints/Creatures/BPP_Creature.CurrentHunger` (+ (`/Game/Blueprints/Creatures/BPP_Creature.CurrentHunger` _asbpp_creature) 50.0) _asbpp_creature)
          (set `/Game/Blueprints/Creatures/BPP_Creature.isSeekingFood` false _asbpp_creature)
          (`self.Wander`))))
    (:`Is Not Valid`
      (`self.SeekFood`))))

(fn `UserConstructionScript`)