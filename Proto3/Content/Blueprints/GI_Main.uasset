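; GI_Main is the game instance that handles saving and loading the game through a BP_SaveGame object in a named slot.
; SaveGameData writes SaveData to the slot and prints success or failure.
; LoadGameData reads the slot, casts to BP_SaveGame, stores it as SaveData and calls LoadSavedData.
; Init, SaveCurrentData and LoadSavedData are still empty stubs.
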(event `self.ReceiveInit`)

(event `/Game/Blueprints/Save-Load/BPI_SaveGame.SaveGameData`
  ; Save Game Data
  (bind _returnvalue (`GameplayStatics.SaveGameToSlot` (`self.SaveData`) (`self.Slot Name`)))
  (if _returnvalue
    (`KismetSystemLibrary.PrintString` "Save Success")
    (else
      (`KismetSystemLibrary.PrintString` "Save Failed"))))

(event `/Game/Blueprints/Save-Load/BPI_SaveGame.LoadGameData`
  ; Load Game Data
  (bind _returnvalue (`GameplayStatics.LoadGameFromSlot` (`self.Slot Name`)))
  (bind _asbp_save_game (cast `/Game/Blueprints/Save-Load/BP_SaveGame` _returnvalue))
  (set `self.SaveData` _asbp_save_game)
  (`self.Load Saved Data`))

(fn `Load Saved Data`)

(fn `Save Current Data`)